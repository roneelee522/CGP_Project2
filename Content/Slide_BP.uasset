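; Slide zone that sends the SideScrollerCharacter sliding while it overlaps a Box trigger.
; Entering removes friction and braking, raises speed limits, pushes velocity toward negative Y while zeroing X and Z, disables input, and plays slide animation and sound.
; Leaving restores hardcoded movement values and the character's NormalSpeed, then returns input and Animation Blueprint mode after a short delay.
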(event `self.Box.OnComponentBeginOverlap`
  (params (OverlappedComponent :type "PrimitiveComponent Object Reference") (OtherActor :type "Actor Object Reference") (OtherComp :type "PrimitiveComponent Object Reference") (OtherBodyIndex :type Integer) (bFromSweep :type Boolean) (SweepResult :type "HitResult Structure (by ref)"))
  (bind _asside_scroller_character (cast `/Game/SideScrollerBP/Blueprints/SideScrollerCharacter` OtherActor))
  (bind _charactermovement (`Character.CharacterMovement` _asside_scroller_character))
  (set `CharacterMovementComponent.BrakingDecelerationWalking` 0.0 _charactermovement)
  (set `CharacterMovementComponent.GroundFriction` 0.0 _charactermovement)
  (set `CharacterMovementComponent.MaxAcceleration` 20000.0 _charactermovement)
  (set `CharacterMovementComponent.MaxWalkSpeed` 2000.0 _charactermovement)
  (bind (_velocity_x _velocity_y) (`KismetMathLibrary.BreakVector` (`MovementComponent.Velocity` _charactermovement)))
  (set `MovementComponent.Velocity` (`KismetMathLibrary.MakeVector` 0.0 (+ _velocity_y -300.0)) _charactermovement)
  (`self.DisableInput` _asside_scroller_character null)
  (`SkeletalMeshComponent.PlayAnimation` (`Character.Mesh` _asside_scroller_character) "/Game/Mannequin/Character/character_slide.character_slide" false)
  (`GameplayStatics.PlaySoundAtLocation` "/Game/sound/slide_audio.slide_audio" (`SceneComponent.K2_GetComponentLocation` (`self.StaticMesh`)) (struct) 1.0 1.0 0.0 null null null))

(event `self.Box.OnComponentEndOverlap`
  (params (OverlappedComponent :type "PrimitiveComponent Object Reference") (OtherActor :type "Actor Object Reference") (OtherComp :type "PrimitiveComponent Object Reference") (OtherBodyIndex :type Integer))
  (bind _asside_scroller_character (cast `/Game/SideScrollerBP/Blueprints/SideScrollerCharacter` OtherActor))
  (bind _charactermovement (`Character.CharacterMovement` _asside_scroller_character))
  (set `CharacterMovementComponent.BrakingDecelerationWalking` 2048.0 _charactermovement)
  (set `CharacterMovementComponent.GroundFriction` 8.0 _charactermovement)
  (set `CharacterMovementComponent.MaxAcceleration` 2000.0 _charactermovement)
  (set `CharacterMovementComponent.MaxWalkSpeed` (`/Game/SideScrollerBP/Blueprints/SideScrollerCharacter.NormalSpeed` _asside_scroller_character) _charactermovement)
  (`KismetSystemLibrary.Delay` 0.5)
  (`self.EnableInput` _asside_scroller_character null)
  (`SkeletalMeshComponent.SetAnimationMode` (`Character.Mesh` _asside_scroller_character) "AnimationBlueprint"))

(fn `UserConstructionScript`)