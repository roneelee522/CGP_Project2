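; Intermittent gust-of-wind hazard that launches any side-scroller character entering its box, using a vertical velocity of jump velocity minus a large offset (normally downward).
; A looping timer periodically opens a short gap by disabling the box's overlap events and hiding the particle effect, then restores both after a delay.
; The launch overrides the character's existing Z velocity; the end-overlap handler only casts and has no effect.
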(event `self.ReceiveBeginPlay`
  (`KismetSystemLibrary.K2_SetTimerDelegate` (delegate `windegap`) 4.0 true))

(event `windegap`
  (bind _particlesystem (`self.ParticleSystem`))
  (bind _box_collision (`self.Box Collision`))
  (set `PrimitiveComponent.bGenerateOverlapEvents` false _box_collision)
  (`SceneComponent.SetVisibility` _particlesystem false false)
  (`KismetSystemLibrary.Delay` 1.5)
  (set `PrimitiveComponent.bGenerateOverlapEvents` true _box_collision)
  (`SceneComponent.SetVisibility` _particlesystem true false)
  (`ActorComponent.SetActive` _particlesystem true false))

(event `self.Box Collision.OnComponentBeginOverlap`
  (params (OverlappedComponent :type "PrimitiveComponent Object Reference") (OtherActor :type "Actor Object Reference") (OtherComp :type "PrimitiveComponent Object Reference") (OtherBodyIndex :type Integer) (bFromSweep :type Boolean) (SweepResult :type "HitResult Structure (by ref)"))
  (bind _asside_scroller_character (cast `/Game/SideScrollerBP/Blueprints/SideScrollerCharacter` OtherActor))
  (`Character.LaunchCharacter` _asside_scroller_character (`KismetMathLibrary.MakeVector` 0.0 0.0 (+ (`CharacterMovementComponent.JumpZVelocity` (`Character.CharacterMovement` _asside_scroller_character)) -2000.0)) false true))

(event `self.Box Collision.OnComponentEndOverlap`
  (params (OverlappedComponent :type "PrimitiveComponent Object Reference") (OtherActor :type "Actor Object Reference") (OtherComp :type "PrimitiveComponent Object Reference") (OtherBodyIndex :type Integer))
  (cast `/Game/SideScrollerBP/Blueprints/SideScrollerCharacter` OtherActor))

(fn `UserConstructionScript`)